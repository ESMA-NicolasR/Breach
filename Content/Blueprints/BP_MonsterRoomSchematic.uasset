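; BP_MonsterRoomSchematic is a schematic of the monster room that shows a gauge for each exit: window, door, vents and pits.
; On BeginPlay it maps each exit location enum to the WBP_Gauge hosted by its widget component.
; Public functions look up a gauge by location to update its progress or play its warning or neutral state.
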(event EventBeginPlay
  (CallFunction|InitMap))

(event Collision|EventActorBeginOverlap
  (params (OtherActor :type Actor%20Object%20Reference)))

(event EventTick
  (params (DeltaSeconds :type Float%20%28single-precision%29)))

(fn ConstructionScript)

(fn UpdateProgressforExit
  (params (Location :type E_SymbolLocation%20Enum :default "NewEnumerator0") (Progress :type Float%20%28double-precision%29))
  (Default|UpdateProgress (.Value (Utilities|Map|Find (Variables|Default|GetGaugeMap) Location)) Progress))

(fn InitMap
  (Utilities|FlowControl|Sequence
    (:then_0
      (Utilities|Map|Add (Variables|Default|GetGaugeMap) "NewEnumerator0" (.AsWBP%20Gauge (Utilities|Casting|CastToWBP_Gauge (UserInterface|GetWidget (Variables|Default|GetWindowWidget))))))
    (:then_1
      (Utilities|Map|Add (Variables|Default|GetGaugeMap) "NewEnumerator1" (.AsWBP%20Gauge (Utilities|Casting|CastToWBP_Gauge (UserInterface|GetWidget (Variables|Default|GetVentGroundWidget))))))
    (:then_2
      (Utilities|Map|Add (Variables|Default|GetGaugeMap) "NewEnumerator2" (.AsWBP%20Gauge (Utilities|Casting|CastToWBP_Gauge (UserInterface|GetWidget (Variables|Default|GetDoorWidget))))))
    (:then_3
      (Utilities|Map|Add (Variables|Default|GetGaugeMap) "NewEnumerator3" (.AsWBP%20Gauge (Utilities|Casting|CastToWBP_Gauge (UserInterface|GetWidget (Variables|Default|GetPitGroundWidget))))))
    (:then_4
      (Utilities|Map|Add (Variables|Default|GetGaugeMap) "NewEnumerator4" (.AsWBP%20Gauge (Utilities|Casting|CastToWBP_Gauge (UserInterface|GetWidget (Variables|Default|GetPitCeilingWidget))))))
    (:then_5
      (Utilities|Map|Add (Variables|Default|GetGaugeMap) "NewEnumerator5" (.AsWBP%20Gauge (Utilities|Casting|CastToWBP_Gauge (UserInterface|GetWidget (Variables|Default|GetVentWallWidget))))))
    (:then_6
      (Utilities|Map|Add (Variables|Default|GetGaugeMap) "NewEnumerator6" (.AsWBP%20Gauge (Utilities|Casting|CastToWBP_Gauge (UserInterface|GetWidget (Variables|Default|GetVentCeilingWidget))))))))

(fn WarningforExit
  (params (Location :type E_SymbolLocation%20Enum :default "NewEnumerator0"))
  (Default|PlayWarning (.Value (Utilities|Map|Find (Variables|Default|GetGaugeMap) Location))))

(fn NeutralforExit
  (params (Location :type E_SymbolLocation%20Enum :default "NewEnumerator0"))
  (Default|PlayNeutral (.Value (Utilities|Map|Find (Variables|Default|GetGaugeMap) Location))))