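; Gravity system manager component that plays a gravity effect and relocates the monster to an exit.
; StartGravityEffect activates a VFX component and sets its world rotation to the given rotation.
; ApplyGravityToMonster stuns the monster, waits briefly, then moves it without sweep to the MonsterAnchor of the exit looked up by location in the player controller's ExitsMap.
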(event Custom|StartGravityEffect
  (params (Rotation :type Rotator))
  (bind _vfxtostart (Variables|Default|GetVFXToStart))
  (Components|Activation|Activate _vfxtostart true)
  (Transformation|SetWorldRotation _vfxtostart Rotation false false))

(event Custom|ApplyGravityToMonster
  (params (Location :type E_SymbolLocation%20Enum :default "NewEnumerator0"))
  (bind _monster (CallFunction|GetMonsterCharacter))
  (Default|GetStunned _monster)
  (Utilities|FlowControl|Delay 1.0)
  (Transformation|SetActorLocation _monster (Transformation|GetWorldLocation (Variables|/Game/Blueprints/BP_Exit.BP_Exit_C|GetMonsterAnchor (.Value (Utilities|Map|Find (Variables|/Game/Blueprints/BP_PlayerController.BP_PlayerController_C|GetExitsMap (CallFunction|GetPlayerController)) Location)))) false false))

(event EventBeginPlay)

(event EventTick
  (params (DeltaSeconds :type Float%20%28single-precision%29)))