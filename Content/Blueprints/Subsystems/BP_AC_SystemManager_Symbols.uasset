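; Actor component that manages console symbol input, matching entered patterns to symbols and pairs of symbols to launchable combinations.
; On BeginPlay it builds lookup maps from the available symbols and combinations, keyed by converted pattern and combination index.
; Confirmed patterns fill two symbol slots with console UI LED feedback, and the second starts the combo animation.
; CheckCombo launches a matching combination or signals failure, then resets and calls LookAtConsole.
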(event EventBeginPlay
  (Variables|Default|SetPlayerController (CallFunction|GetPlayerController))
  (CallFunction|InitSymbols))

(event EventTick
  (params (DeltaSeconds :type Float%20%28single-precision%29)))

(fn ResetCombo
  (Variables|Default|SetFirstSymbol 0)
  (Variables|Default|SetSecondSymbol 0))

(fn InitSymbols
  (Utilities|FlowControl|Sequence
    (:then_0
      (for _array_element (Variables|Default|GetAvailableSymbols)
        (Utilities|Map|Add (Variables|Default|GetSymbolsMap) (CallFunction|ConvertPattern (Variables|/Game/Blueprints/Symbols/Single/BP_DA_Symbol.BP_DA_Symbol_C|GetPattern _array_element)) _array_element)))
    (:then_1
      (for _array_element_2 (Variables|Default|GetAvailableCombinations)
        (Utilities|Map|Add (Variables|Default|GetCombinationsMap) (CallFunction|GetCombinationIndexfromAsset _array_element_2) _array_element_2)))))

(fn TryConfirmPattern
  (params (Pattern :type Array%20of%20Booleans))
  (bind _code (CallFunction|ConvertPattern Pattern))
  (bind _symbolsmap (Variables|Default|GetSymbolsMap))
  (bind (_value _returnvalue) (Utilities|Map|Find _symbolsmap _code))
  (if _returnvalue
    (CallFunction|ConfirmSymbol _value)
    (Default|ConfirmCells (Variables|/Game/Blueprints/BP_PlayerController.BP_PlayerController_C|GetConsoleUI (Variables|Default|GetPlayerController)) _value)
    (else
      (Default|CancelCells (Variables|/Game/Blueprints/BP_PlayerController.BP_PlayerController_C|GetConsoleUI (Variables|Default|GetPlayerController))))))

(fn ConfirmSymbol
  (params (Symbol :type BP%20DA%20Symbol%20Object%20Reference))
  (Variables|Default|GetFirstSymbol
    (:then
      (Default|OkLed2 (Variables|/Game/Blueprints/BP_PlayerController.BP_PlayerController_C|GetConsoleUI (Variables|Default|GetPlayerController)))
      (Variables|Default|SetSecondSymbol Symbol)
      (Default|StartComboAnimation (Variables|Default|GetPlayerController)))
    (:else
      (Default|OkLed1 (Variables|/Game/Blueprints/BP_PlayerController.BP_PlayerController_C|GetConsoleUI (Variables|Default|GetPlayerController)))
      (Variables|Default|SetFirstSymbol Symbol))))

(fn CancelSymbols
  (Default|CancelCells (Variables|/Game/Blueprints/BP_PlayerController.BP_PlayerController_C|GetConsoleUI (Variables|Default|GetPlayerController)))
  (Variables|Default|GetFirstSymbol
    (:then
      (Default|ErrorLed1 (Variables|/Game/Blueprints/BP_PlayerController.BP_PlayerController_C|GetConsoleUI (Variables|Default|GetPlayerController)))
      (Variables|Default|SetFirstSymbol 0))
    (:else)))

(fn CheckCombo
  (bind _combinationsmap (Variables|Default|GetCombinationsMap))
  (bind _firstsymbol (Variables|Default|GetFirstSymbol))
  (bind _secondsymbol (Variables|Default|GetSecondSymbol))
  (bind _index (CallFunction|GetCombinationIndexfromSymbols _firstsymbol _secondsymbol))
  (bind (_value _returnvalue) (Utilities|Map|Find _combinationsmap _index))
  (LocalVariables|SetFoundCombination _value)
  (if _returnvalue
    (Default|ComboOK (Variables|/Game/Blueprints/BP_PlayerController.BP_PlayerController_C|GetConsoleUI (Variables|Default|GetPlayerController)))
    (Default|Launch (LocalVariables|GetFoundCombination) (Variables|Default|GetPlayerController))
    (CallFunction|ResetCombo)
    (Default|LookatConsole (Variables|/Game/Blueprints/BP_PlayerController.BP_PlayerController_C|GetCurrentConsole (Variables|Default|GetPlayerController)))
    (else
      (Default|ComboKO (Variables|/Game/Blueprints/BP_PlayerController.BP_PlayerController_C|GetConsoleUI (Variables|Default|GetPlayerController)))
      (CallFunction|ResetCombo)
      (Default|LookatConsole (Variables|/Game/Blueprints/BP_PlayerController.BP_PlayerController_C|GetCurrentConsole (Variables|Default|GetPlayerController))))))