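; Actor component that manages a one-shot laser defense aimed at one of an ordered list of exit locations.
; MoveUp and MoveDown step a clamped index through that list to set the current location.
; Fire works once: if the monster's current exit matches, it damages and stuns the monster; otherwise it deals that exit's full max health as damage to it.
; Results are reported through debug prints.
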(event EventBeginPlay)

(event EventTick
  (params (DeltaSeconds :type Float%20%28single-precision%29)))

(fn MoveUp
  (CallFunction|ChangePosition (+ (Variables|Default|GetCurrentLocationIndex) 1)))

(fn MoveDown
  (CallFunction|ChangePosition (- (Variables|Default|GetCurrentLocationIndex) 1)))

(fn Fire
  (bind _monster (CallFunction|GetMonsterCharacter))
  (bind _asbpplayercontroller (CallFunction|GetPlayerController))
  (bind _currentlocation (Variables|Default|GetCurrentLocation))
  (bind _exitsmap (Variables|/Game/Blueprints/BP_PlayerController.BP_PlayerController_C|GetExitsMap _asbpplayercontroller))
  (bind _value (Utilities|Map|Find _exitsmap _currentlocation))
  (if (Variables|Default|GetHasFired)
    (Development|PrintString "Laser already used")
    (else
      (Variables|Default|SetHasFired true)
      (if (Utilities|Enum|Equal(Enum) (Variables|/Game/Blueprints/BP_Exit.BP_Exit_C|GetLocation (Variables|/Game/Blueprints/BP_MonsterCharacter.BP_MonsterCharacter_C|GetCurrentExit (CallFunction|GetMonsterCharacter))) (Variables|Default|GetCurrentLocation))
        (Development|PrintString "Laser Success")
        (Default|LoseHealth _monster 2.0)
        (Default|GetStunned _monster)
        (else
          (Development|PrintString "Laser fail")
          (Default|LoseHp _value (Variables|/Game/Blueprints/BP_Exit.BP_Exit_C|GetMaxHealth _value)))))))

(fn ChangePosition
  (params (Index :type Integer))
  (bind _output_get (Variables|Default|SetCurrentLocationIndex (Math|Integer|Clamp(Integer) Index 0 (- (Utilities|Array|Length (Variables|Default|GetLocationsOrder)) 1))))
  (bind _output_get_2 (Variables|Default|SetCurrentLocation (Utilities|Array|Get(acopy) (Variables|Default|GetLocationsOrder) _output_get)))
  (Development|PrintString (Utilities|String|Append "Current laser location : " (Utilities|String|EnumtoString _output_get_2))))