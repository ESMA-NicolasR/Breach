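; Temperature system manager component that tracks a temperature value per location and breaks that location's exit when it swings too far.
; Fire raises and frost lowers the stored value, then both run a shared break check.
; Once the absolute value exceeds the threshold, the check deals max-health damage to the exit found in the player controller's ExitsMap.
; Each check also prints the absolute temperature for debugging.
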(event EventBeginPlay)

(event EventTick
  (params (DeltaSeconds :type Float%20%28single-precision%29)))

(fn FireonLocation
  (params (Location :type E_SymbolLocation%20Enum%20%28by%20ref%29 :default "NewEnumerator0"))
  (Utilities|Map|Add (Variables|Default|GetLocationsMap) Location (+ (.Value (Utilities|Map|Find (Variables|Default|GetLocationsMap) Location)) 1))
  (CallFunction|CheckLocationIsBroken Location))

(fn FrostonLocation
  (params (Location :type E_SymbolLocation%20Enum%20%28by%20ref%29 :default "NewEnumerator0"))
  (Utilities|Map|Add (Variables|Default|GetLocationsMap) Location (- (.Value (Utilities|Map|Find (Variables|Default|GetLocationsMap) Location)) 1))
  (CallFunction|CheckLocationIsBroken Location))

(fn CheckLocationIsBroken
  (params (Location :type E_SymbolLocation%20Enum :default "NewEnumerator0"))
  (bind _asbpplayercontroller (CallFunction|GetPlayerController))
  (bind _locationsmap (Variables|Default|GetLocationsMap))
  (bind _value (Utilities|Map|Find _locationsmap Location))
  (bind _exitsmap (Variables|/Game/Blueprints/BP_PlayerController.BP_PlayerController_C|GetExitsMap _asbpplayercontroller))
  (bind _returnvalue (Math|Integer|Absolute(Integer) _value))
  (bind _value_2 (Utilities|Map|Find _exitsmap Location))
  (Development|PrintString (Utilities|String|Append "Temperature on " (Utilities|String|EnumtoString Location) " = " (Utilities|String|ToString(Integer) _returnvalue)))
  (if (> _returnvalue 2)
    (Default|LoseHp _value_2 (Variables|/Game/Blueprints/BP_Exit.BP_Exit_C|GetMaxHealth _value_2))))