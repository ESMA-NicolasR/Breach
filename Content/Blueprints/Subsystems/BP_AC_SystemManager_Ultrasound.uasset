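; Actor component that manages the ultrasound system, switching the UltrasoundMachine's emission on and off and stunning the monster.
; ActivateUltrasounds checks IsFrequencyOk, then starts emission and immediately calls GetStunned on the monster character.
; IsFrequencyOk always returns true, so activation is currently unconditional.
; DeactivateUltrasounds only stops emission, and the event graph has no active logic.
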(event EventBeginPlay)

(event EventTick
  (params (DeltaSeconds :type Float%20%28single-precision%29)))

(fn ActivateUltrasounds
  (if (CallFunction|IsFrequencyOk)
    (Default|StartEmitting (Variables|Default|GetUltrasoundMachine))
    (Default|GetStunned (CallFunction|GetMonsterCharacter))))

(fn IsFrequencyOk
  (return true))

(fn DeactivateUltrasounds
  (Default|StopEmitting (Variables|Default|GetUltrasoundMachine)))