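; Manager actor that holds back experience content until StartExperience is called, registering itself on the player controller as StartExperienceManager.
; On BeginPlay it finds tagged lights and posters, plus the ultrasound machine and monster room schematic, then hides or disables them.
; It also swaps the tagged console's symbol and combination arrays with its starting sets, delayed one tick.
; StartExperience reveals everything and swaps the symbols back.
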(event EventBeginPlay
  (Variables|/Game/Blueprints/BP_PlayerController.BP_PlayerController_C|SetStartExperienceManager (CallFunction|GetPlayerController) self)
  (Utilities|FlowControl|Sequence
    (:then_0
      (Lights|InitLights)
      (Lights|LightsOff))
    (:then_1
      (Posters|InitPosters)
      (Posters|PostersOff))
    (:then_2
      (Symbols|InitSymbols)
      ;[0.15 0.15 0.15 0.5] Don't interfere with other component begin play
      (Utilities|FlowControl|DelayUntilNextTick)
      (Symbols|SymbolsSwap))
    (:then_3
      (Ultrasounds|InitUltrasounds)
      (Ultrasounds|UltrasoundsDisable))
    (:then_4
      (Schematics|InitSchematics)
      (Schematics|SchematicsOff))))

(fn ConstructionScript)

(fn InitLights
  (bind _outactors (Actor|GetAllActorsOfClasswithTag "/Script/Engine.Light" "ExperienceLight"))
  (for _array_element _outactors
    (Utilities|Array|Add (Variables|Default|GetLights) (Variables|/Script/Engine.Light|GetLightComponent _array_element))))

(fn LightsOff
  (for _array_element (Variables|Default|GetLights)
    (Rendering|SetVisibility _array_element false false)))

(fn Lightson
  (for _array_element (Variables|Default|GetLights)
    (Rendering|SetVisibility _array_element true false)))

(fn InitPosters
  (bind _outactors (Actor|GetAllActorsOfClasswithTag "/Game/Blueprints/BP_InteractiblePoster.BP_InteractiblePoster_C" "ExperiencePoster"))
  (for _array_element _outactors
    (Utilities|Array|Add (Variables|Default|GetPosters) _array_element)))

(fn PostersOff
  (for _array_element (Variables|Default|GetPosters)
    (Rendering|SetActorHiddenInGame _array_element true)
    (Collision|SetActorEnableCollision _array_element false)))

(fn Posterson
  (for _array_element (Variables|Default|GetPosters)
    (Rendering|SetActorHiddenInGame _array_element false)
    (Collision|SetActorEnableCollision _array_element true)))

(fn InitSymbols
  (bind _outactors (Actor|GetAllActorsOfClasswithTag "/Game/Blueprints/BP_InteractibleConsole.BP_InteractibleConsole_C" "ExperienceConsole"))
  (Variables|Default|SetSymbolsManager (Variables|/Game/Blueprints/BP_InteractibleConsole.BP_InteractibleConsole_C|GetBP_AC_SystemManager_Symbols (Utilities|Array|Get(acopy) _outactors))))

(fn SymbolsSwap
  (Utilities|FlowControl|Sequence
    (:then_0
      ;[0.15 0.15 0.15 0.5] Swap symbols arrays
      (Variables|Default|SetTmpSymbols (Variables|/Game/Blueprints/Subsystems/BP_AC_SystemManager_Symbols.BP_AC_SystemManager_Symbols_C|GetAvailableSymbols (Variables|Default|GetSymbolsManager)))
      (Variables|/Game/Blueprints/Subsystems/BP_AC_SystemManager_Symbols.BP_AC_SystemManager_Symbols_C|SetAvailableSymbols (Variables|Default|GetSymbolsManager) (Variables|Default|GetStartSymbols))
      (Variables|Default|SetStartSymbols (Variables|Default|GetTmpSymbols)))
    (:then_1
      ;[0.15 0.15 0.15 0.5] Swap combinations arrays
      (Variables|Default|SetTmpCombinations (Variables|/Game/Blueprints/Subsystems/BP_AC_SystemManager_Symbols.BP_AC_SystemManager_Symbols_C|GetAvailableCombinations (Variables|Default|GetSymbolsManager)))
      (Variables|/Game/Blueprints/Subsystems/BP_AC_SystemManager_Symbols.BP_AC_SystemManager_Symbols_C|SetAvailableCombinations (Variables|Default|GetSymbolsManager) (Variables|Default|GetStartCombinations))
      (Variables|Default|SetStartCombinations (Variables|Default|GetTmpCombinations)))
    (:then_2
      ;[0.15 0.15 0.15 0.5] Recompute maps for symbols
      (Default|InitSymbols (Variables|Default|GetSymbolsManager)))))

(fn StartExperience
  (Lights|Lightson)
  (Posters|Posterson)
  (Symbols|SymbolsSwap)
  (Ultrasounds|UltrasoundsEnable)
  (Schematics|Schematicson))

(fn UltrasoundsEnable
  (bind _ultrasounds (Variables|Default|GetUltrasounds))
  (Rendering|SetActorHiddenInGame _ultrasounds false)
  (Collision|SetActorEnableCollision _ultrasounds true))

(fn UltrasoundsDisable
  (bind _ultrasounds (Variables|Default|GetUltrasounds))
  (Rendering|SetActorHiddenInGame _ultrasounds true)
  (Collision|SetActorEnableCollision _ultrasounds false))

(fn InitUltrasounds
  (bind _returnvalue (Actor|GetActorOfClass "/Game/Blueprints/BP_UltrasoundMachine.BP_UltrasoundMachine_C"))
  (Variables|Default|SetUltrasounds _returnvalue))

(fn InitSchematics
  (bind _returnvalue (Actor|GetActorOfClass "/Game/Blueprints/BP_MonsterRoomSchematic.BP_MonsterRoomSchematic_C"))
  (Variables|Default|SetSchematics _returnvalue))

(fn SchematicsOff
  (Rendering|SetActorHiddenInGame (Variables|Default|GetSchematics) true))

(fn Schematicson
  (Rendering|SetActorHiddenInGame (Variables|Default|GetSchematics) false))