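; Player controller for a console-driven game where drawn symbol pairs launch combinations, also handling camera movement and the win/lose screens.
; It creates the movement and console widgets, and Tick forwards the buffered move intention to the character camera once it can accept one.
; Nine-cell patterns resolve to symbols through a lookup map; two confirmed symbols trigger an animation, with CheckCombo launching any matching combination.
; Exits begin self-damage after startup and stop on win or loss.
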(event Custom|StartComboAnimation
  (Utilities|FlowControl|Delay 0.5)
  (Default|StartCheckCombo (Variables|Default|GetConsoleUI)))

(event Custom|Move
  (params (Direction :type Integer))
  (Variables|Default|SetIntentionMove Direction)
  (Components|Timeline|PlayfromStart (Variables|Default|GetInputBuffering)))

(event EventBeginPlay
  (CallFunction|InitUI)
  (Symbols|InitSymbols)
  (Utilities|FlowControl|Delay 0.2)
  (CallFunction|InitExits))

(event EventTick
  (params (DeltaSeconds :type Float%20%28single-precision%29))
  (bind _asbp_character_camera (CallFunction|GetCharacterCamera))
  (bind _intentionmove (Variables|Default|GetIntentionMove))
  (if (and (>= _intentionmove 0) (Variables|/Game/Blueprints/Bp_CharacterCamera.Bp_CharacterCamera_C|GetCanPressMove (CallFunction|GetCharacterCamera)))
    (Variables|/Game/Blueprints/Bp_CharacterCamera.Bp_CharacterCamera_C|SetCanPressMove (CallFunction|GetCharacterCamera) false)
    (Development|PrintString (Utilities|String|ToString(Integer) _intentionmove))
    (switch int _intentionmove
      (:0
        (Default|MoveForwards _asbp_character_camera))
      (:1
        (Default|MoveBackwards _asbp_character_camera))
      (:2
        (Default|MoveLeft _asbp_character_camera))
      (:3
        (Default|MoveRight _asbp_character_camera))
      (:4
        (Default|TurnLeft _asbp_character_camera))
      (:5
        (Default|TurnRight _asbp_character_camera)))))

(fn ConstructionScript)

(fn FlipCell
  (params (Index :type Integer))
  (if (and (Variables|Default|GetIsDrawing) (not (Utilities|Array|Get(acopy) (Variables|Default|GetUsedCells) Index)))
    (Utilities|Array|SetArrayElem (Variables|Default|GetUsedCells) Index true)
    (Default|Flip (.AsWBP%20Console%20Cell (Utilities|Casting|CastToWBP_ConsoleCell (Class|PanelWidget|GetChildat (Variables|/Game/Blueprints/UI/WBP_ConsolePad.WBP_ConsolePad_C|GetCells (Variables|Default|GetConsoleUI)) Index))))))

(fn StartDrawing
  (Variables|Default|SetIsDrawing true)
  (Cells|CleanCells))

(fn StopDrawing
  (Variables|Default|SetIsDrawing false))

(fn CleanCells
  (Variables|Default|SetUsedCells (Utilities|Array|MakeArray false false false false false false false false false)))

(fn TryConfirmPattern
  (params (Pattern :type Array%20of%20Booleans))
  (bind _code (CallFunction|ConvertPattern Pattern))
  (bind _symbolsmap (Variables|Default|GetSymbolsMap))
  (bind (_value _returnvalue) (Utilities|Map|Find _symbolsmap _code))
  (if _returnvalue
    (Symbols|ConfirmSymbol _value)
    (Default|ConfirmCells (Variables|Default|GetConsoleUI) _value)
    (else
      (Default|CancelCells (Variables|Default|GetConsoleUI)))))

(fn InitUI
  (Utilities|FlowControl|Sequence
    (:then_0
      (bind _returnvalue (UserInterface|CreateWidget "/Game/Blueprints/UI/Bp_WID_CharacterMovement.Bp_WID_CharacterMovement_C" self))
      (bind _output_get (Variables|Default|SetMovementUI _returnvalue))
      (UserInterface|Viewport|AddtoViewport _output_get 0))
    (:then_1
      (bind _returnvalue_2 (UserInterface|CreateWidget "/Game/Blueprints/UI/WBP_ConsolePad.WBP_ConsolePad_C" self))
      (bind _output_get_2 (Variables|Default|SetConsoleUI _returnvalue_2)))
    (:then_2
      (Input|SetInputModeUIOnly self 0 "DoNotLock" false))))

(fn InitSymbols
  (Utilities|FlowControl|Sequence
    (:then_0
      (for _array_element (Variables|Default|GetAvailableSymbols)
        (Utilities|Map|Add (Variables|Default|GetSymbolsMap) (CallFunction|ConvertPattern (Variables|/Game/Blueprints/Symbols/Single/BP_DA_Symbol.BP_DA_Symbol_C|GetPattern _array_element)) _array_element)))
    (:then_1
      (for _array_element_2 (Variables|Default|GetAvailableCombinations)
        (Utilities|Map|Add (Variables|Default|GetCombinationsMap) (CallFunction|GetCombinationIndexfromAsset _array_element_2) _array_element_2)))))

(fn ConfirmSymbol
  (params (Symbol :type BP%20DA%20Symbol%20Object%20Reference))
  (Variables|Default|GetFirstSymbol
    (:then
      (Default|OkLed2 (Variables|Default|GetConsoleUI))
      (Variables|Default|SetSecondSymbol Symbol)
      (CallFunction|StartComboAnimation))
    (:else
      (Default|OkLed1 (Variables|Default|GetConsoleUI))
      (Variables|Default|SetFirstSymbol Symbol))))

(fn CancelSymbols
  (Default|CancelCells (Variables|Default|GetConsoleUI))
  (Variables|Default|GetFirstSymbol
    (:then
      (Default|ErrorLed1 (Variables|Default|GetConsoleUI))
      (Variables|Default|SetFirstSymbol 0))
    (:else)))

(fn CheckCombo
  (bind _combinationsmap (Variables|Default|GetCombinationsMap))
  (bind _firstsymbol (Variables|Default|GetFirstSymbol))
  (bind _secondsymbol (Variables|Default|GetSecondSymbol))
  (bind _index (CallFunction|GetCombinationIndexfromSymbols _firstsymbol _secondsymbol))
  (bind (_value _returnvalue) (Utilities|Map|Find _combinationsmap _index))
  (LocalVariables|SetFoundCombination _value)
  (if _returnvalue
    (Default|ComboOK (Variables|Default|GetConsoleUI))
    (Default|Launch (LocalVariables|GetFoundCombination) (CallFunction|GetConsoleController))
    (Symbols|ResetCombo)
    (else
      (Default|ComboKO (Variables|Default|GetConsoleUI))
      (Symbols|ResetCombo))))

(fn ResetCombo
  (Variables|Default|SetFirstSymbol 0)
  (Variables|Default|SetSecondSymbol 0))

(fn LoseGame
  (CallFunction|StopExits)
  (Widget|RemovefromParent (Variables|Default|GetConsoleUI))
  (bind _returnvalue (UserInterface|CreateWidget "/Game/Blueprints/UI/WBP_EcranMort.WBP_EcranMort_C" self))
  (UserInterface|Viewport|AddtoViewport _returnvalue 0))

(fn WinGame
  (CallFunction|StopExits)
  (Widget|RemovefromParent (Variables|Default|GetConsoleUI))
  (bind _returnvalue (UserInterface|CreateWidget "/Game/Blueprints/UI/WBP_EcranWin.WBP_EcranWin_C" (Game|GetPlayerController 0)))
  (UserInterface|Viewport|AddtoViewport _returnvalue 0))

(fn InitExits
  (for _array_element (Variables|Default|GetExits)
    (Default|StartSelfDamage _array_element)))

(fn StopExits
  (for _array_element (Variables|Default|GetExits)
    (Default|StopSelfDamage _array_element)))