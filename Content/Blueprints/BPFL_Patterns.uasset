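; Blueprint function library that converts patterns into integer codes and builds lookup keys for symbol combinations.
; ConvertPattern packs a boolean array into a bitmask integer, adding two to the power of each true element's index.
; GetCombinationIndex sorts two symbol enum names alphabetically and concatenates them, so the string key is independent of symbol order.
; Two wrappers derive that key from a combination asset or from two symbols.
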(fn ConvertPattern
  (params (Pattern :type Array%20of%20Booleans))
  (LocalVariables|SetTMPCode 0)
  (for (_array_element _array_index) Pattern
    (LocalVariables|SetTMPCode (select _array_element (Math|Float|Truncate (+ (Math|Float|Power 2.0 (Math|Conversions|ToFloat(Integer) _array_index)) (LocalVariables|GetTMPCode))) (LocalVariables|GetTMPCode))))
  (return (LocalVariables|GetTMPCode)))

(fn GetCombinationIndexfromAsset
  (params (Combination :type BP%20DA%20Symbol%20Combination%20Object%20Reference))
  (return (CallFunction|GetCombinationIndex (Variables|/Game/Blueprints/Symbols/Combination/BP_DA_SymbolCombination.BP_DA_SymbolCombination_C|GetSymbol1 Combination) (Variables|/Game/Blueprints/Symbols/Combination/BP_DA_SymbolCombination.BP_DA_SymbolCombination_C|GetSymbol2 Combination))))

(fn GetCombinationIndexfromSymbols
  (params (Symbol1 :type BP%20DA%20Symbol%20Object%20Reference) (Symbol2 :type BP%20DA%20Symbol%20Object%20Reference))
  (return (CallFunction|GetCombinationIndex (Variables|/Game/Blueprints/Symbols/Single/BP_DA_Symbol.BP_DA_Symbol_C|GetName Symbol1) (Variables|/Game/Blueprints/Symbols/Single/BP_DA_Symbol.BP_DA_Symbol_C|GetName Symbol2))))

(fn GetCombinationIndex
  (params (SymbolName1 :type E_SymbolName%20Enum :default "NewEnumerator0") (SymbolName2 :type E_SymbolName%20Enum :default "NewEnumerator0"))
  (bind _output_get (LocalVariables|SetTmpArray (Utilities|Array|MakeArray (Utilities|String|EnumtoString SymbolName1) (Utilities|String|EnumtoString SymbolName2))))
  (Class|KismetArrayLibrary|SortStringArray _output_get)
  (return (Utilities|String|Append (Utilities|Array|Get(acopy) (LocalVariables|GetTmpArray)) (Utilities|Array|Get(acopy) (LocalVariables|GetTmpArray) 1))))