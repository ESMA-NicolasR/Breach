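; Blueprint function library of global getters for the game's player controller, player character, monster and game instance.
; Player getters cast the index 0 controller and character to project classes, and the monster is read from that controller's Monster variable.
; A helper converts a movement input enum into a world direction from the player character's control rotation forward and right vectors, negated for backwards and left.
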(fn GetPlayerController
  (bind _asbp_player_controller (Utilities|Casting|CastToBP_PlayerController (Game|GetPlayerController 0)))
  (return _asbp_player_controller))

(fn GetPlayerCharacter
  (bind _asbp_player_character (Utilities|Casting|CastToBP_PlayerCharacter (Game|GetPlayerCharacter 0)))
  (return _asbp_player_character))

(fn GetWorldDirectionfromInput
  (params (Input :type E_PlayerInput%20Enum :default "NewEnumerator6"))
  (switch Utilities|FlowControl|Switch|SwitchonE_PlayerInput Input
    (:NewEnumerator0
      (return (Math|Vector|GetForwardVector (Pawn|GetControlRotation (CallFunction|GetPlayerCharacter) :!class /Script/Engine.Pawn))))
    (:NewEnumerator1
      (return (Math|Vector|NegateVector (Math|Vector|GetForwardVector (Pawn|GetControlRotation (CallFunction|GetPlayerCharacter) :!class /Script/Engine.Pawn)))))
    (:NewEnumerator2
      (return (Math|Vector|NegateVector (Math|Vector|GetRightVector (Pawn|GetControlRotation (CallFunction|GetPlayerCharacter) :!class /Script/Engine.Pawn)))))
    (:NewEnumerator3
      (return (Math|Vector|GetRightVector (Pawn|GetControlRotation (CallFunction|GetPlayerCharacter) :!class /Script/Engine.Pawn))))))

(fn GetMonsterCharacter
  (return (Variables|/Game/Blueprints/BP_PlayerController.BP_PlayerController_C|GetMonster (CallFunction|GetPlayerController))))

(fn GetGameInstance
  (return (.AsBP%20Game%20Instance (Utilities|Casting|CastToBP_GameInstance (Game|GetGameInstance)))))