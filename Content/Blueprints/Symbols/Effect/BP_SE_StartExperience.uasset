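; BP_SE_StartExperience is a symbol effect that, when cast, starts the game experience through the controller.
; On the LaunchCasted event it calls StartExperience on the controller's experience manager.
; It then moves the Monster to the MonsterAnchor transform found in the controller's exits map for the Location key and triggers ReceiveAttack on it with a fixed attack type.
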(event EventLaunchCasted
  (params (Controller :type BP%20Player%20Controller%20Object%20Reference))
  (bind _location (Variables|Default|GetLocation))
  (bind _monster (Variables|/Game/Blueprints/BP_PlayerController.BP_PlayerController_C|GetMonster Controller))
  (bind _exitsmap (Variables|/Game/Blueprints/BP_PlayerController.BP_PlayerController_C|GetExitsMap Controller))
  (bind _value (Utilities|Map|Find _exitsmap _location))
  (bind _monsteranchor (Variables|/Game/Blueprints/BP_Exit.BP_Exit_C|GetMonsterAnchor _value))
  (Default|StartExperience (Variables|/Game/Blueprints/BP_PlayerController.BP_PlayerController_C|GetStartExperienceManager Controller))
  (Transformation|SetActorLocationAndRotation _monster (Transformation|GetWorldLocation _monsteranchor) (Transformation|GetWorldRotation _monsteranchor))
  (Default|ReceiveAttack _monster "NewEnumerator4"))