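; BP_SE_Stun is a symbol effect that stuns the monster when cast at the location of its current exit.
; On LaunchCasted, it prints a debug string with its element, location and duration.
; It then calls GetStunned on the controller's monster if that monster has a valid current exit matching the effect's location.
; Element and Duration appear only in the debug print and are not passed to the stun.
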(event EventLaunchCasted
  (params (Controller :type BP%20Player%20Controller%20Object%20Reference))
  (bind _monster (Variables|/Game/Blueprints/BP_PlayerController.BP_PlayerController_C|GetMonster Controller))
  (Development|PrintString 0 (Utilities|String|Append "Stun (" (Utilities|String|EnumtoString (Variables|Default|GetElement)) ") on " (Utilities|String|EnumtoString (Variables|Default|GetLocation)) " for " (Utilities|String|ToString(Float) (Variables|Default|GetDuration))))
  (bind _currentexit (Variables|/Game/Blueprints/BP_MonsterCharacter.BP_MonsterCharacter_C|GetCurrentExit _monster)
    (:then
      (if (Utilities|Enum|Equal(Enum) (Variables|/Game/Blueprints/BP_Exit.BP_Exit_C|GetLocation _currentexit) (Variables|Default|GetLocation))
        (Default|GetStunned _monster)))
    (:else)))