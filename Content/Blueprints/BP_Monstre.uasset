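; BP_Monstre is a monster actor with win and death outcomes: player overlap with its Box stops the Death timeline and shows the win screen.
; Both outcomes call PeutCeDeplacer on the player character before adding their widget.
; Two countdown-to-death versions exist, a Death timeline calling MortDuJoueur and a Couldown event decrementing Decomptes.
; BeginPlay is empty and the timeline and looping-timer starts are unconnected, so neither countdown starts here.
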(event OnComponentBeginOverlap(Box)
  (params (OverlappedComponent :type Primitive%20Component%20Object%20Reference) (OtherActor :type Actor%20Object%20Reference) (OtherComp :type Primitive%20Component%20Object%20Reference) (OtherBodyIndex :type Integer) (bFromSweep :type Boolean) (SweepResult :type Hit%20Result%20Structure%20%28by%20ref%29))
  (if (== OtherActor (Game|GetPlayerCharacter 0))
    (Audio|Components|Audio|Stop (Variables|Default|GetDeath))
    (bind _asbp_dm_third_person_character (Utilities|Casting|CastToBP_DM_ThirdPersonCharacter (Game|GetPlayerCharacter 0)))
    (Default|PeutCeDeplacer _asbp_dm_third_person_character)
    (bind _returnvalue (UserInterface|CreateWidget "/Game/Blueprints/UI/WBP_EcranWin.WBP_EcranWin_C" (Game|GetPlayerController 0)))
    (UserInterface|Viewport|AddtoViewport _returnvalue 0)))

(event Custom|Couldown
  (bind _output_get (Variables|Default|Setdecomptes (Math|Float|Clamp(Float) (- (Variables|Default|Getdecomptes) (Variables|Default|Getcentiemes)) 0.0 (Variables|Default|Getdecomptes))))
  (Development|PrintText (Utilities|Text|ToText(String) (Class|KismetStringLibrary|TimeSecondstoString _output_get)))
  (if (== (Variables|Default|Getdecomptes) 0.0)
    (bind _asbp_dm_third_person_character (Utilities|Casting|CastToBP_DM_ThirdPersonCharacter (Game|GetPlayerCharacter 0)))
    (Default|PeutCeDeplacer _asbp_dm_third_person_character)
    (bind _returnvalue (UserInterface|CreateWidget "/Game/Blueprints/UI/WBP_EcranMort.WBP_EcranMort_C" (Game|GetPlayerController 0)))
    (UserInterface|Viewport|AddtoViewport _returnvalue 0)))

(event EventBeginPlay)

(fn ConstructionScript)

(fn MortDuJoueur
  (bind _asbp_dm_third_person_character (Utilities|Casting|CastToBP_DM_ThirdPersonCharacter (Game|GetPlayerCharacter 0)))
  (Default|PeutCeDeplacer _asbp_dm_third_person_character)
  (bind _returnvalue (UserInterface|CreateWidget "/Game/Blueprints/UI/WBP_EcranMort.WBP_EcranMort_C" (Game|GetPlayerController 0)))
  (UserInterface|Viewport|AddtoViewport _returnvalue 0))