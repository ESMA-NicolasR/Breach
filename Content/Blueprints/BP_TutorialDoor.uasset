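; Two-part sliding tutorial door that registers itself on BeginPlay with the tutorial-door system manager found through the player controller.
; Open and Close play or reverse a timeline that lerps both parts between their start and end marker components.
; Both also post a Wwise event on the player character, choosing the open or closed switch from the DoorOpen flag before updating it, with debug prints.
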(event EventBeginPlay
  (Utilities|FlowControl|Sequence
    (:then_0
      (Variables|/Game/Blueprints/Subsystems/BP_AC_SystemManager_TutorialDoor.BP_AC_SystemManager_TutorialDoor_C|SetDoor (Variables|/Game/Blueprints/BP_PlayerController.BP_PlayerController_C|GetBP_AC_SystemManager_TutorialDoor (CallFunction|GetPlayerController)) self))))

(fn ConstructionScript)

(fn Open
  (Audio|Components|Audio|Play (Variables|Default|GetAnimationTimeline))
  (CallFunction|WwiseSoundDoorOpen)
  (Variables|Default|SetDoorOpen true))

(fn Close
  (Utilities|String|Reverse (Variables|Default|GetAnimationTimeline))
  (CallFunction|WwiseSoundDoorOpen)
  (Variables|Default|SetDoorOpen false))

(fn WwiseSoundDoorOpen
  (bind _asbpplayercharacter (CallFunction|GetPlayerCharacter))
  (if (Variables|Default|GetDoorOpen)
    ;[0.15 0.15 0.15 0.5] DoorClosed
    (Class|AkGameplayStatics|SetSwitch "/Game/WwiseAudio/Switches/Default_Work_Unit/Door/STDR_Door-ST_DoorClosed.STDR_Door-ST_DoorClosed" _asbpplayercharacter)
    (Class|AkGameplayStatics|PostEvent "/Game/WwiseAudio/Events/Default_Work_Unit/Ambiant/Event_DoorTutorial.Event_DoorTutorial" _asbpplayercharacter)
    (Development|PrintString "ClosedDoor")
    (else
      ;[0.15 0.15 0.15 0.5] DoorOpen
      (Class|AkGameplayStatics|SetSwitch "/Game/WwiseAudio/Switches/Default_Work_Unit/Door/STDR_Door-ST_DoorOpen.STDR_Door-ST_DoorOpen" _asbpplayercharacter)
      (Class|AkGameplayStatics|PostEvent "/Game/WwiseAudio/Events/Default_Work_Unit/Ambiant/Event_DoorTutorial.Event_DoorTutorial" _asbpplayercharacter)
      (Development|PrintString "OpenDoor"))))