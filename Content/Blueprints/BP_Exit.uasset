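; BP_Exit is a destructible exit that registers itself in the player controller's AvailableExits list and tracks its own health.
; Damage through LoseHp clamps health and pushes its fraction to MonsterRoomSchematic as progress for that exit's Location, with debug prints.
; When health reaches zero, Destroy calls MonsterKillPlayer on the player controller, so a broken exit means the monster kills the player.
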(event EventBeginPlay
  (Utilities|Array|Add (Variables|/Game/Blueprints/BP_PlayerController.BP_PlayerController_C|GetAvailableExits (CallFunction|GetPlayerController)) self)
  (Variables|Default|SetHealth (Variables|Default|GetMaxHealth))
  (Utilities|FlowControl|Delay 0.2)
  (CallFunction|UpdateHealthDisplay))

(event Collision|EventActorBeginOverlap
  (params (OtherActor :type Actor%20Object%20Reference)))

(event EventTick
  (params (DeltaSeconds :type Float%20%28single-precision%29)))

(fn ConstructionScript)

(fn LoseHp
  (params (Damage :type Float%20%28double-precision%29))
  (CallFunction|ChangeHealth (- (Variables|Default|GetHealth) Damage)))

(fn ChangeHealth
  (params (NewHealth :type Float%20%28double-precision%29))
  (bind _output_get (Variables|Default|SetHealth (Math|Float|Clamp(Float) NewHealth 0.0 (Variables|Default|GetMaxHealth))))
  (CallFunction|UpdateHealthDisplay)
  (if (<= _output_get 0.0)
    (CallFunction|Destroy)))

(fn UpdateHealthDisplay
  (Development|PrintString (Utilities|String|Append (Utilities|String|EnumtoString (Variables|Default|GetLocation)) ": " (Utilities|String|ToString(Float) (Variables|Default|GetHealth)) " health remaining"))
  (Default|UpdateProgressforExit (Variables|Default|GetMonsterRoomSchematic) (Variables|Default|GetLocation) (/ (Variables|Default|GetHealth) (Variables|Default|GetMaxHealth))))

(fn Destroy
  (Development|PrintString (Utilities|String|Append (Utilities|String|EnumtoString (Variables|Default|GetLocation)) " destroyed"))
  (Default|MonsterKillPlayer (CallFunction|GetPlayerController)))