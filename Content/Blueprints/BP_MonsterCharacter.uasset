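; BP_MonsterCharacter is the enemy monster that attacks the player's exits, with its health shown on a gauge actor.
; A behaviour state machine, paced by a rate-scaled timeline as timer, picks an exit, drains its HP and recovers from stuns.
; Elemental hits query a resistance component to damage, stun or be resisted, with stuns sending it back to spawn.
; Zero health wins the game, while KillPlayer stages a timed death sequence that ends in a loss.
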(event OnActorBeginOverlap(TriggerMonstreStart)
  (params (OverlappedActor :type Actor%20Object%20Reference) (OtherActor :type Actor%20Object%20Reference))
  ;[0.15 0.15 0.15 0.5] Alternative to BP_StartExperience
)

(event Custom|Start%20DelayMonstre
  (Timeline|StartDelayTimeline Play
    (:Finished
      (CallFunction|Rotationplayer)
      (bind _asbp_attack_player (Utilities|Casting|CastToBP_AttackPlayer (Variables|Default|GetSpawnAtack)))
      (Default|AttackPlayer _asbp_attack_player))))

(event Custom|StartDelayPlayer
  (bind _asbpplayercontroller (CallFunction|GetPlayerController))
  (Timeline|StartDelayTimeline2 Play
    (:Finished
      (Default|LoseGame _asbpplayercontroller)
      (Game|Feedback|ClientPlayForceFeedback _asbpplayercontroller "/Game/ForceFeedbacks/FFE_Wrong.FFE_Wrong" "None" false false false))))

(event EventBeginPlay
  (CallFunction|InitGaugeMonster)
  (Variables|/Game/Blueprints/BP_PlayerController.BP_PlayerController_C|SetMonster (CallFunction|GetPlayerController) self)
  (Variables|Default|SetHealth (Variables|Default|GetMaxHealth))
  (CallFunction|UpdateHealthDisplay))

(fn ConstructionScript)

(fn StartAttackingExit
  (params (Exit :type BP%20Exit%20Object%20Reference))
  (bind _output_get (Variables|Default|SetCurrentExit Exit))
  (Variables|Default|SetAirborne (Variables|/Game/Blueprints/BP_Exit.BP_Exit_C|GetMonsterAirborne _output_get))
  (Default|WarningHealth _output_get)
  (Transformation|SetActorLocationAndRotation (Transformation|GetWorldLocation (Variables|/Game/Blueprints/BP_Exit.BP_Exit_C|GetMonsterAnchor _output_get)) (Transformation|GetWorldRotation (Variables|/Game/Blueprints/BP_Exit.BP_Exit_C|GetMonsterAnchor _output_get)))
  (Default|ShowEmergencyLight (CallFunction|GetPlayerController))
  (Class|AkGameplayStatics|PostEvent "/Game/WwiseAudio/Events/Default_Work_Unit/Monster/Event_MonsterHurt.Event_MonsterHurt" (CallFunction|GetMonsterCharacter)))

(fn MakeDecision
  (switch Utilities|FlowControl|Switch|SwitchonE_MonsterBehaviour (Variables|Default|GetBehaviour)
    (:NewEnumerator0
      (Development|PrintString "Taking action")
      (bind _exit (CallFunction|ChooseExit))
      (CallFunction|StartAttackingExit _exit)
      (Variables|Default|SetBehaviour "NewEnumerator1")
      (CallFunction|WaitNextDecision (Variables|Default|GetTimeBetweenAttacks)))
    (:NewEnumerator1
      (Development|PrintString "Attacking Exit")
      (Default|LoseHp (Variables|Default|GetCurrentExit) 1.0)
      (CallFunction|WaitNextDecision (Variables|Default|GetTimeBetweenAttacks)))
    (:NewEnumerator2
      (Development|PrintString "End stun")
      (Variables|Default|SetBehaviour "NewEnumerator0")
      (CallFunction|WaitNextDecision (Variables|Default|GetTimeBetweenActions)))))

(fn WaitNextDecision
  (params (Time :type Float%20%28double-precision%29))
  (bind _decisiontimeline (Variables|Default|GetDecisionTimeline))
  (Components|Timeline|SetPlayRate _decisiontimeline (/ 1.0 Time))
  (Components|Timeline|PlayfromStart _decisiontimeline))

(fn ReceiveAttack
  (params (Element :type E_SymbolElement%20Enum :default "NewEnumerator0"))
  (bind _reaction (Default|GetReaction (Variables|Default|GetBP_AC_MonsterResistances) Element))
  (switch Utilities|FlowControl|Switch|SwitchonE_ResistanceLevel _reaction
    (:NewEnumerator0
      (Development|PrintString "Damage")
      (CallFunction|GetStunned 0.0)
      (CallFunction|LoseHealth 1.0))
    (:NewEnumerator1
      (Development|PrintString "Stun")
      (CallFunction|GetStunned (Variables|Default|GetResistStunDuration)))
    (:NewEnumerator2
      (Development|PrintString "No effect")
      (Variables|Default|SetResist true)
      (Class|KismetSystemLibrary|SetTimerforNextTickDelegate (EventDispatchers|CreateEvent :!event EndResist)))))

(fn LoseHealth
  (params (Damage :type Float%20%28double-precision%29))
  (CallFunction|ChangeHealth (- (Variables|Default|GetHealth) Damage))
  (Class|AkGameplayStatics|PostEvent (Variables|Wwise|GetAKMonsterHurt)))

(fn GetStunned
  (params (OverrideStunDuration :type Float%20%28double-precision%29))
  (bind _spawnpoint (Variables|Default|GetSpawnPoint))
  (|HandleCurrentExit)
  (Transformation|SetActorLocationAndRotation (Transformation|GetActorLocation _spawnpoint) (Transformation|GetActorRotation _spawnpoint))
  (Variables|Default|SetBehaviour "NewEnumerator2")
  (CallFunction|WaitNextDecision (Math|Float|SelectFloat OverrideStunDuration (Variables|Default|GetBaseStunDuration) (!= OverrideStunDuration 0.0)))
  (Default|HideEmergencyLight (CallFunction|GetPlayerController)))

(fn ChooseExit
  (if (Variables|Default|GetIsFirstAttack)
    (Variables|Default|SetIsFirstAttack false)
    (return (.Value (Utilities|Map|Find (Variables|/Game/Blueprints/BP_PlayerController.BP_PlayerController_C|GetExitsMap (CallFunction|GetPlayerController)) "NewEnumerator0")))
    (else
      (return (.OutItem (Utilities|Array|Random (Variables|/Game/Blueprints/BP_PlayerController.BP_PlayerController_C|GetAvailableExits (CallFunction|GetPlayerController))))))))

(fn ChangeHealth
  (params (NewHealth :type Float%20%28double-precision%29))
  (bind _output_get (Variables|Default|SetHealth (Math|Float|Clamp(Float) NewHealth 0.0 (Variables|Default|GetMaxHealth))))
  (CallFunction|UpdateHealthDisplay)
  (if (<= _output_get 0.0)
    (CallFunction|Die)))

(fn UpdateHealthDisplay
  (Default|UpdateMonsterGauge (Variables|Default|GetGaugeMonster) (/ (Variables|Default|GetHealth) (Variables|Default|GetMaxHealth)))
  (Development|PrintString (Utilities|String|Append "Monster health : " (Utilities|String|ToString(Float) (Variables|Default|GetHealth)))))

(fn Die
  (Development|PrintString "Monster is dead")
  (Variables|Default|SetBehaviour "NewEnumerator3")
  (Default|WinGame (CallFunction|GetPlayerController)))

(fn KillPlayer
  (bind _spawnatack (Variables|Default|GetSpawnAtack))
  (bind _spot_attack_player (Variables|Default|GetSpot%20Attack%20Player))
  (Transformation|SetActorLocation (CallFunction|GetPlayerCharacter) (Transformation|GetActorLocation _spot_attack_player) false false)
  (Pawn|SetControlRotation (CallFunction|GetPlayerController) (Transformation|GetActorRotation _spot_attack_player))
  (Transformation|SetActorLocationAndRotation (Transformation|GetActorLocation _spawnatack) (Transformation|GetActorRotation _spawnatack))
  (Game|Player|SetViewTargetwithBlend (CallFunction|GetPlayerController) (Variables|Default|GetSpawnAtack) 0.3 "VTBlend_Cubic" 0.0 false)
  (CallFunction|StartDelayMonstre)
  (Variables|Default|SetBehaviour "NewEnumerator4"))

(fn Rotationplayer
  (Components|Animation|PlayAnimation (Variables|/Script/Engine.Character|GetMesh (CallFunction|GetPlayerCharacter)) "/Game/Characters/Mannequins/Anims/Death/MM_Death_Front_02.MM_Death_Front_02" false)
  (CallFunction|StartDelayPlayer))

(fn InitGaugeMonster
  (bind _returnvalue (Actor|GetActorOfClass "/Game/Blueprints/BP_GaugeMonster.BP_GaugeMonster_C"))
  (Variables|Default|SetGaugeMonster _returnvalue))

(fn EndResist
  (Variables|Default|SetResist false))