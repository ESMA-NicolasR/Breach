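; Actor component that tracks a monster's resistance to each symbol element and adapts it as the monster is hit with that element.
; On BeginPlay it fills the Resistances map with Weak for every E_SymbolElement value.
; GetReaction returns the current level for the given element, then raises the stored level one step from Weak through Medium to High, where it stays.
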(event EventBeginPlay
  (CallFunction|InitResistances))

(event EventTick
  (params (DeltaSeconds :type Float%20%28single-precision%29)))

(fn InitResistances
  (bind _enumvalue (|ForEachE_SymbolElement)
    (:LoopBody
      (Utilities|Map|Add (Variables|Default|GetResistances) _enumvalue "NewEnumerator0"))))

(fn GetReaction
  (params (Element :type E_SymbolElement%20Enum :default "NewEnumerator0"))
  (switch Utilities|FlowControl|Switch|SwitchonE_ResistanceLevel (.Value (Utilities|Map|Find (Variables|Default|GetResistances) Element))
    (:NewEnumerator0
      (Utilities|Map|Add (Variables|Default|GetResistances) Element "NewEnumerator1")
      (return "NewEnumerator0"))
    (:NewEnumerator1
      (Utilities|Map|Add (Variables|Default|GetResistances) Element "NewEnumerator2")
      (return "NewEnumerator1"))
    (:NewEnumerator2
      (return "NewEnumerator2"))))