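; Interactable console Blueprint that lets the player use a console UI and switch views between the console and a combo result.
; Starting or ending interaction toggles the character's interact state and the controller's console display, and registers or clears itself as current console.
; A dynamic pad material created at BeginPlay reflects open state through a scalar parameter.
; Look-at functions blend the view to itself, showing the UI panel, or to a second camera.
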(event EventBeginPlay
  (|CallParentFunction)
  (bind _returnvalue (Rendering|Material|CreateDynamicMaterialInstance (Variables|Default|GetCube) 0 "/Game/Materials/M_Pad.M_Pad" "None" :!class /Script/Engine.PrimitiveComponent))
  (Variables|Default|SetMaterial _returnvalue))

(event Collision|EventActorBeginOverlap
  (params (OtherActor :type Actor%20Object%20Reference)))

(event EventTick
  (params (DeltaSeconds :type Float%20%28single-precision%29)))

(fn ConstructionScript
  (|CallParentFunction))

(fn StartInteraction
  (bind _asbpplayercontroller (CallFunction|GetPlayerController))
  (|CallParentFunction)
  (Default|StartInteract (CallFunction|GetPlayerCharacter))
  (Default|ShowConsole _asbpplayercontroller)
  (Variables|/Game/Blueprints/BP_PlayerController.BP_PlayerController_C|SetCurrentConsole _asbpplayercontroller self)
  (Rendering|Material|SetScalarParameterValue (Variables|Default|GetMaterial) "IsOpen" 1.0 :!class /Script/Engine.MaterialInstanceDynamic))

(fn EndInteraction
  (bind _asbpplayercontroller (CallFunction|GetPlayerController))
  (|CallParentFunction)
  (Default|StopInteract (CallFunction|GetPlayerCharacter))
  (Default|HideConsole _asbpplayercontroller)
  (Variables|/Game/Blueprints/BP_PlayerController.BP_PlayerController_C|SetCurrentConsole _asbpplayercontroller 0)
  (Rendering|Material|SetScalarParameterValue (Variables|Default|GetMaterial) "IsOpen" 0.0 :!class /Script/Engine.MaterialInstanceDynamic))

(fn LookatComboResult
  (Game|Player|SetViewTargetwithBlend (CallFunction|GetPlayerController) (Variables|Default|GetSecondCamera) 0.3 "VTBlend_Cubic" 0.0 false))

(fn LookatConsole
  (bind _asbpplayercontroller (CallFunction|GetPlayerController))
  (Game|Player|SetViewTargetwithBlend _asbpplayercontroller self 0.5 "VTBlend_Cubic" 0.0 false)
  (Default|ShowPanel (Variables|/Game/Blueprints/BP_PlayerController.BP_PlayerController_C|GetConsoleUI _asbpplayercontroller)))