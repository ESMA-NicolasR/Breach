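; Blueprint that plays surface-dependent Wwise footstep sounds for the player character.
; Its FootStepsWwiseDetection event traces 100 units down from BP_PlayerCharacter on the Visibility channel to read the physical surface.
; The surface selects a blood or concrete switch, defaulting to concrete, which is set on the player before the footstep event posts.
; It also prints the selected switch name for debugging.
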(event Custom|FootStepsWwiseDetection
  (bind _asbpplayercharacter (CallFunction|GetPlayerCharacter))
  ;[0.15 0.15 0.15 0.5] WwiseFootSteps
  (bind _returnvalue (Actor|GetActorOfClass "/Game/Blueprints/BP_PlayerCharacter.BP_PlayerCharacter_C"))
  (bind _outhit (Collision|LineTraceByChannel (Transformation|GetActorLocation _returnvalue) (- (Transformation|GetActorLocation _returnvalue) "0.000000,0.000000,100.000000") "TraceTypeQuery1" false 0 "None"))
  (Class|AkGameplayStatics|SetSwitch (Utilities|Select :Index (Collision|GetSurfaceType _outhit) :SurfaceType_Default "/Game/WwiseAudio/Switches/Default_Work_Unit/GroundSurface/STFT_GroundSurface-ST_Concrete.STFT_GroundSurface-ST_Concrete" :SurfaceType1 "/Game/WwiseAudio/Switches/Default_Work_Unit/GroundSurface/STFT_GroundSurface-ST_Blood.STFT_GroundSurface-ST_Blood" :SurfaceType2 "/Game/WwiseAudio/Switches/Default_Work_Unit/GroundSurface/STFT_GroundSurface-ST_Concrete.STFT_GroundSurface-ST_Concrete") _asbpplayercharacter)
  (Class|AkGameplayStatics|PostEvent "/Game/WwiseAudio/Events/Default_Work_Unit/Character/Event_CharacterFootSteps.Event_CharacterFootSteps" _asbpplayercharacter)
  (Development|PrintString (Utilities|GetDisplayName (Utilities|Select :Index (Collision|GetSurfaceType _outhit) :SurfaceType_Default "/Game/WwiseAudio/Switches/Default_Work_Unit/GroundSurface/STFT_GroundSurface-ST_Concrete.STFT_GroundSurface-ST_Concrete" :SurfaceType1 "/Game/WwiseAudio/Switches/Default_Work_Unit/GroundSurface/STFT_GroundSurface-ST_Blood.STFT_GroundSurface-ST_Blood" :SurfaceType2 "/Game/WwiseAudio/Switches/Default_Work_Unit/GroundSurface/STFT_GroundSurface-ST_Concrete.STFT_GroundSurface-ST_Concrete"))))