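; Character camera Blueprint that moves its actor in fixed-length steps forward, backward, left or right, relative to its facing.
; Each direction event first runs a debug-drawn Visibility line trace, and a hit blocks the step and re-enables CanPressMove.
; A clear path plays the matching walk animation and starts MovingTimeline, scaled by TimeToMove.
; The timeline lerps the actor's location to the target without sweeping, then sets CanPressMove on finish.
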(event Custom|Up
  (CallFunction|TryMoveTowards (Transformation|GetActorForwardVector) "/Game/Characters/Mannequins/Anims/Unarmed/Walk/MF_Unarmed_Walk_Fwd.MF_Unarmed_Walk_Fwd"))

(event Custom|Down
  (CallFunction|TryMoveTowards (Math|Vector|NegateVector (Transformation|GetActorForwardVector)) "/Game/Characters/Mannequins/Anims/Unarmed/Walk/MF_Unarmed_Walk_Bwd.MF_Unarmed_Walk_Bwd"))

(event Custom|Left
  (CallFunction|TryMoveTowards (Math|Vector|NegateVector (Transformation|GetActorRightVector)) "/Game/Characters/Mannequins/Anims/Unarmed/Walk/MF_Unarmed_Walk_Left.MF_Unarmed_Walk_Left"))

(event Custom|Right
  (CallFunction|TryMoveTowards (Transformation|GetActorRightVector) "/Game/Characters/Mannequins/Anims/Unarmed/Walk/MF_Unarmed_Walk_Right.MF_Unarmed_Walk_Right"))

(event EventBeginPlay
  (Components|Timeline|SetPlayRate (Variables|Default|GetMovingTimeline) (/ 1.0 (Variables|Default|GetTimeToMove))))

(fn ConstructionScript)

(fn MoveTowards
  (params (AnimToPlay :type Animation%20Asset%20Object%20Reference) (Direction :type Vector))
  (Components|Animation|PlayAnimation (Variables|Character|GetMesh) AnimToPlay false)
  (bind _output_get (Variables|Default|SetStartPosition (Transformation|GetActorLocation)))
  (Variables|Default|SetTargetPosition (+ _output_get (* Direction (Variables|Default|GetStepLength))))
  (Components|Timeline|PlayfromStart (Variables|Default|GetMovingTimeline)))

(fn CheckWallDirection
  (params (Direction :type Vector))
  (bind _returnvalue (Transformation|GetActorLocation))
  (bind _returnvalue_2 (Collision|LineTraceByChannel _returnvalue (+ _returnvalue (* Direction (Variables|Default|GetWallCheckDistance))) "TraceTypeQuery1" false 0 "ForDuration"))
  (if _returnvalue_2
    (Development|PrintString "Hit")
    (return true)
    (else
      (Development|PrintString "Miss")
      (return false))))

(fn TryMoveTowards
  (params (Direction :type Vector) (AnimToPlay :type Animation%20Asset%20Object%20Reference))
  (bind _hit (CallFunction|CheckWallDirection Direction))
  (if _hit
    (Variables|Default|SetCanPressMove true)
    (Development|PrintString "Movement impossible")
    (else
      (CallFunction|MoveTowards AnimToPlay Direction))))