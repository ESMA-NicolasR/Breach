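; Interactable ultrasound machine that toggles an emission to stun the monster, and destroys a designated exit once its cumulative active time runs out.
; It registers with the player controller's ultrasound system manager on BeginPlay.
; Toggling plays or pauses a timeline rate-scaled to TimeToDestroy, stuns the monster for the remaining time or resets its decision wait, and updates the label.
; The timeline drives the countdown text and, on finish, deals max-health damage to the exit.
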(event EventBeginPlay
  (|CallParentFunction)
  (Components|Timeline|SetPlayRate (Variables|Default|GetDamagingTimeline) (/ 1.0 (Variables|Default|GetTimeToDestroy)))
  (CallFunction|UpdateTextwithTimeLeft)
  (Variables|/Game/Blueprints/Subsystems/BP_AC_SystemManager_Ultrasound.BP_AC_SystemManager_Ultrasound_C|SetUltrasoundMachine (Variables|/Game/Blueprints/BP_PlayerController.BP_PlayerController_C|GetBP_AC_SystemManager_Ultrasound (CallFunction|GetPlayerController)) self))

(event Collision|EventActorBeginOverlap
  (params (OtherActor :type Actor%20Object%20Reference)))

(event EventTick
  (params (DeltaSeconds :type Float%20%28single-precision%29)))

(fn ConstructionScript)

(fn StartEmitting
  (Audio|Components|Audio|Play (Variables|Default|GetDamagingTimeline))
  (Default|GetStunned (CallFunction|GetMonsterCharacter) (CallFunction|GetTimeLeft))
  (Rendering|Components|TextRender|SetText (Variables|Default|GetLabelUse) (Utilities|Text|ToText(String) "Ultrasounds 
ACTIVE")))

(fn StopEmitting
  (Audio|Components|Audio|Stop (Variables|Default|GetDamagingTimeline))
  (Default|WaitNextDecision (CallFunction|GetMonsterCharacter) 0.5)
  (Rendering|Components|TextRender|SetText (Variables|Default|GetLabelUse) (Utilities|Text|ToText(String) "Ultrasounds 
READY")))

(fn UpdateTextwithTimeLeft
  (Rendering|Components|TextRender|SetText (Variables|Default|GetTextTimer) (Utilities|Text|ToText(String) (Utilities|String|Append (Utilities|String|ToString(Text) (Utilities|Text|ToText(Float) (CallFunction|GetTimeLeft) "HalfToEven" false true 1 4 0 2)) "s"))))

(fn DestroyExit
  (bind _asbpplayercontroller (CallFunction|GetPlayerController))
  (bind _exittodestroy (Variables|Default|GetExitToDestroy))
  (bind _exitsmap (Variables|/Game/Blueprints/BP_PlayerController.BP_PlayerController_C|GetExitsMap _asbpplayercontroller))
  (bind _value (Utilities|Map|Find _exitsmap _exittodestroy))
  (Default|LoseHp _value (Variables|/Game/Blueprints/BP_Exit.BP_Exit_C|GetMaxHealth _value)))

(fn GetTimeLeft
  (return (* (- 1.0 (Components|Timeline|GetPlaybackPosition (Variables|Default|GetDamagingTimeline))) (Variables|Default|GetTimeToDestroy))))

(fn StartInteraction
  (|CallParentFunction)
  (bind _output_get (Variables|Default|SetIsEmitting (not (Variables|Default|GetIsEmitting))))
  (if _output_get
    (CallFunction|StartEmitting)
    (else
      (CallFunction|StopEmitting))))