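; BP_FireArm is a turret trap that lowers, sweeps its cannon and attacks the monster, then retracts.
; StartFireSequence sets rotation, ammo state and target locations, then chains timelines for descent, yaw sweep and reversed ascent.
; With ammo, the monster is hit as the sweep starts if its current exit matches a target location, so damage involves no projectile or trace.
; It registers itself with the player controller's FireArm system manager.
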(event EventBeginPlay
  (Components|Timeline|SetPlayRate (Variables|Default|GetVerticalMovement) (/ 1.0 (Variables|Default|GetTimeForVerticalMovement)))
  (Components|Timeline|SetPlayRate (Variables|Default|GetHorizontalSpray) (/ 1.0 (Variables|Default|GetTimeForHorizontalSpray)))
  (Variables|/Game/Blueprints/Subsystems/BP_AC_SystemManager_FireArm.BP_AC_SystemManager_FireArm_C|SetFireArm (Variables|/Game/Blueprints/BP_PlayerController.BP_PlayerController_C|GetBP_AC_SystemManager_FireArm (CallFunction|GetPlayerController)) self))

(event Collision|EventActorBeginOverlap
  (params (OtherActor :type Actor%20Object%20Reference)))

(event EventTick
  (params (DeltaSeconds :type Float%20%28single-precision%29)))

(fn ConstructionScript)

(fn StartFireSequence
  (params (WithAmmo :type Boolean) (NewRotation :type Rotator) (TargetLocations :type Array%20of%20E_SymbolLocation%20Enums :default "NewEnumerator0"))
  (Transformation|SetActorRotation NewRotation)
  (Variables|Default|SetTargetLocations TargetLocations)
  (Variables|Default|SetHasAmmo WithAmmo)
  (CallFunction|GetDown))

(fn GetDown
  (Transformation|SetRelativeRotation (Variables|Default|GetSM_TurretCannon) (Math|Rotator|MakeRotator 0.0 0.0 (Variables|Default|GetAngleAmplitude)) false false)
  (Components|Timeline|PlayfromStart (Variables|Default|GetVerticalMovement)))

(fn GetUp
  (Components|Timeline|ReversefromEnd (Variables|Default|GetVerticalMovement)))

(fn Spray
  (bind _monster (CallFunction|GetMonsterCharacter))
  (Components|Timeline|PlayfromStart (Variables|Default|GetHorizontalSpray))
  (if (Variables|Default|GetHasAmmo)
    (Development|PrintString "Tir à l'arme à feu")
    (for _array_element (Variables|Default|GetTargetLocations)
      (bind _currentexit (Variables|/Game/Blueprints/BP_MonsterCharacter.BP_MonsterCharacter_C|GetCurrentExit _monster)
        (:then
          (if (Utilities|Enum|Equal(Enum) (Variables|/Game/Blueprints/BP_Exit.BP_Exit_C|GetLocation _currentexit) _array_element)
            (Default|ReceiveAttack _monster "NewEnumerator3")))
        (:else)))
    (else
      (Development|PrintString "Clic clic à l'arme à feu"))))