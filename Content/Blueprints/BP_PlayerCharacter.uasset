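; Player character that moves in fixed steps and rotates in quarter turns, reporting to the player controller for input highlighting and move completion.
; A visibility line trace blocks steps into walls, while timelines interpolate location and control yaw over configurable durations.
; A child interactible activator clears collisions when motion starts and searches again when it finishes.
; Interaction functions only set a flag, with animation calls disconnected, and SpawnAttack is empty.
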(event Custom|MoveForwards
  ;[0.15 0.15 0.15 0.5] Movement
  (CallFunction|TryMoveTowards "NewEnumerator0"))

(event Custom|MoveBackwards
  ;[0.15 0.15 0.15 0.5] Movement
  (CallFunction|TryMoveTowards "NewEnumerator1"))

(event Custom|MoveLeft
  ;[0.15 0.15 0.15 0.5] Movement
  (CallFunction|TryMoveTowards "NewEnumerator2"))

(event Custom|MoveRight
  ;[0.15 0.15 0.15 0.5] Movement
  (CallFunction|TryMoveTowards "NewEnumerator3"))

(event Custom|TurnRight
  ;[0.15 0.15 0.15 0.5] Rotation
  (CallFunction|TurnTowards 9e+01 "NewEnumerator5")
  (Default|HighlightPlayerInput (CallFunction|GetPlayerController) "NewEnumerator5"))

(event Custom|TurnLeft
  ;[0.15 0.15 0.15 0.5] Rotation
  (CallFunction|TurnTowards -9e+01 "NewEnumerator4")
  (Default|HighlightPlayerInput (CallFunction|GetPlayerController) "NewEnumerator4"))

(event EventBeginPlay
  ;[0.15 0.15 0.15 0.5] Setup
  (Components|Timeline|SetPlayRate (Variables|Default|GetMovingTimeline) (/ 1.0 (Variables|Default|GetTimeToMove)))
  (Components|Timeline|SetPlayRate (Variables|Default|GetRotatingTimeline) (/ 1.0 (Variables|Default|GetTimeToRotate)))
  (Variables|Default|SetInteractibleActivator (.AsBP%20Interactible%20Activator (Utilities|Casting|CastToBP_InteractibleActivator (Variables|/Script/Engine.ChildActorComponent|GetChildActor (Variables|Default|GetBP_InteractibleActivator))))))

(fn ConstructionScript)

(fn MoveTowards
  (params (Direction :type E_PlayerInput%20Enum :default "NewEnumerator6"))
  (Variables|Animation|SetIsMoving true)
  (Variables|Animation|SetCurrentMovement Direction)
  (bind _output_get (Variables|Movement|SetStartPosition (Transformation|GetActorLocation)))
  (Variables|Movement|SetTargetPosition (+ _output_get (* (CallFunction|GetWorldDirectionfromInput Direction) (Variables|Default|GetStepLength))))
  (Components|Timeline|PlayfromStart (Variables|Default|GetMovingTimeline))
  (Default|HighlightPlayerInput (CallFunction|GetPlayerController) Direction)
  (Default|ClearCollisions (Variables|Default|GetInteractibleActivator)))

(fn CheckWallDirection
  (params (Direction :type E_PlayerInput%20Enum :default "NewEnumerator6"))
  (bind _returnvalue (Transformation|GetActorLocation))
  (bind (_outhit _returnvalue_2) (Collision|LineTraceByChannel _returnvalue (+ _returnvalue (* (CallFunction|GetWorldDirectionfromInput Direction) (Variables|Default|GetWallCheckDistance))) "TraceTypeQuery1" false 0 "ForDuration"))
  (if _returnvalue_2
    (Development|PrintString (Utilities|GetDisplayName (.HitActor (Collision|BreakHitResult _outhit))))
    (return true)
    (else
      (return false))))

(fn TryMoveTowards
  (params (Direction :type E_PlayerInput%20Enum :default "NewEnumerator6"))
  (bind _hit (CallFunction|CheckWallDirection Direction))
  (if _hit
    (Variables|Default|SetCanPressMove true)
    (Development|PrintString "Movement impossible")
    (else
      (CallFunction|MoveTowards Direction))))

(fn TurnTowards
  (params (ZRotation :type Float%20%28double-precision%29) (CurrentMovement :type E_PlayerInput%20Enum :default "NewEnumerator6"))
  (bind _returnvalue (Pawn|GetControlRotation :!class /Script/Engine.Pawn))
  (Variables|Animation|SetIsMoving true)
  (Variables|Animation|SetCurrentMovement CurrentMovement)
  (Variables|Movement|SetStartZRotation (.yaw _returnvalue))
  (Variables|Movement|SetTargetZRotation (+ ZRotation (.yaw _returnvalue)))
  (Components|Timeline|PlayfromStart (Variables|Default|GetRotatingTimeline))
  (Default|ClearCollisions (Variables|Default|GetInteractibleActivator)))

(fn FinishMovement
  (Variables|Default|SetCanPressMove true)
  (Variables|Animation|SetIsMoving false)
  (Default|FinishMovement (CallFunction|GetPlayerController))
  (Default|SearchCollisions (Variables|Default|GetInteractibleActivator)))

(fn SpawnAttack)

(fn StartInteract
  (Variables|Animation|SetIsInteracting true))

(fn StopInteract
  (Variables|Animation|SetIsInteracting false))