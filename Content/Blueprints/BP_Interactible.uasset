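; BP_Interactible is a clickable world object that the player controller can focus on for interaction.
; Clicking its Cube or calling the Click event passes the object to the controller's FocusOnInteractible when IsActivable is set.
; A widget component supplies a WBP_Interactible prompt, hidden at BeginPlay and shown with a looping Floating animation.
; StartInteraction hides that prompt and EndInteraction restores it, both printing debug messages.
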(event OnClicked(Cube)
  (params (TouchedComponent :type Primitive%20Component%20Object%20Reference) (ButtonPressed :type Key%20Structure :default "None"))
  (if (Variables|Default|GetIsActivable)
    (Default|FocusonInteractible (CallFunction|GetPlayerController) self)))

(event Custom|Click
  (if (Variables|Default|GetIsActivable)
    (Default|FocusonInteractible (CallFunction|GetPlayerController) self)))

(event EventBeginPlay
  (bind _aswbp_interactible (Utilities|Casting|CastToWBP_Interactible (UserInterface|GetWidget (Variables|Default|GetInteractibility))))
  (bind _output_get (Variables|Default|SetInteractibilityWidget _aswbp_interactible))
  (Widget|SetVisibility _output_get "Hidden"))

(fn ConstructionScript)

(fn StartInteraction
  (Development|PrintString "Start interact")
  (CallFunction|HideInteractionSprite))

(fn EndInteraction
  (Development|PrintString "End interact")
  (CallFunction|ShowInteractionSprite))

(fn ShowInteractionSprite
  (bind _interactibilitywidget (Variables|Default|GetInteractibilityWidget))
  (Widget|SetVisibility _interactibilitywidget "Visible")
  (UserInterface|Animation|PlayAnimation _interactibilitywidget (Variables|/Game/Blueprints/UI/Feedback/WBP_Interactible.WBP_Interactible_C|GetFloating _interactibilitywidget) 0.0 0 "Forward" 1.0 false))

(fn HideInteractionSprite
  (bind _interactibilitywidget (Variables|Default|GetInteractibilityWidget))
  (Widget|SetVisibility _interactibilitywidget "Hidden")
  (Class|UserWidget|StopAnimation _interactibilitywidget (Variables|/Game/Blueprints/UI/Feedback/WBP_Interactible.WBP_Interactible_C|GetFloating _interactibilitywidget)))