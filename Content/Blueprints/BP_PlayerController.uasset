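; Player controller for a touch-driven, step-movement game, managing movement input, interactable focus, UI screens and win/lose display.
; Movement presses are buffered with a timeline and dispatched to the character when it can move, then wall checks restrict the pad's directions.
; Tapped interactables are clicked via trace; focusing blends the camera and swaps widgets.
; It also drives the console's cell-drawing combo and spawns VFX at mapped exits' monster anchors.
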(event Custom|StartComboAnimation
  (Widget|RemovefromParent (Variables|Default|GetExitFocusUI))
  (Utilities|FlowControl|Delay 0.5)
  (Default|StartCheckCombo (Variables|Default|GetConsoleUI))
  (Default|LookatComboResult (Variables|Default|GetCurrentConsole)))

(event EventBeginPlay
  (CallFunction|InitUI)
  (Components|Timeline|SetPlayRate (Variables|Default|GetInputBuffering) (/ 1.0 (Variables|Inputs|GetInputBufferTime)))
  (Utilities|FlowControl|Delay 0.2)
  (Exits|InitExits))

(event Input|TouchEvents|InputTouch
  (params (Location :type Vector) (FingerIndex :type ETouchIndex%20Enum))
  (:Pressed
    (bind _asbp_interactible (Utilities|Casting|CastToBP_Interactible (.HitActor (Collision|BreakHitResult (.HitResult (Class|PlayerController|GetHitResultUnderFingerbyChannel "Touch1" "TraceTypeQuery1" true))))))
    (Default|Click _asbp_interactible)))

(fn ConstructionScript)

(fn FlipCell
  (params (Index :type Integer))
  (if (and (Variables|Default|GetIsDrawing) (not (Utilities|Array|Get(acopy) (Variables|Default|GetUsedCells) Index)))
    (Utilities|Array|SetArrayElem (Variables|Default|GetUsedCells) Index true)
    (Default|Flip (.AsWBP%20Console%20Cell (Utilities|Casting|CastToWBP_ConsoleCell (Class|PanelWidget|GetChildat (Variables|/Game/Blueprints/UI/WBP_ConsolePad.WBP_ConsolePad_C|GetCells (Variables|Default|GetConsoleUI)) Index))))))

(fn StartDrawing
  (Variables|Default|SetIsDrawing true)
  (Cells|CleanCells))

(fn StopDrawing
  (Variables|Default|SetIsDrawing false))

(fn CleanCells
  (Variables|Default|SetUsedCells (Utilities|Array|MakeArray false false false false false false false false false)))

(fn InitUI
  (Utilities|FlowControl|Sequence
    (:then_0
      (bind _returnvalue (UserInterface|CreateWidget "/Game/Blueprints/UI/WBP_CharacterMovement.WBP_CharacterMovement_C" self))
      (bind _output_get (Variables|Default|SetMovementUI _returnvalue))
      (UserInterface|Viewport|AddtoViewport _output_get 0))
    (:then_1
      (bind _returnvalue_2 (UserInterface|CreateWidget "/Game/Blueprints/UI/WBP_ConsolePad.WBP_ConsolePad_C" self))
      (bind _output_get_2 (Variables|Default|SetConsoleUI _returnvalue_2)))
    (:then_2
      (bind _returnvalue_3 (UserInterface|CreateWidget "/Game/Blueprints/UI/WBP_ExitFocus.WBP_ExitFocus_C" self))
      (Variables|Default|SetExitFocusUI _returnvalue_3))
    (:then_3
      (Input|SetInputModeGameandUI self 0 "DoNotLock" false false))))

(fn LoseGame
  (Widget|RemovefromParent (Variables|Default|GetConsoleUI))
  (Widget|RemovefromParent (Variables|Default|GetMovementUI))
  (bind _returnvalue (UserInterface|CreateWidget "/Game/Blueprints/UI/WBP_LoseScreen.WBP_LoseScreen_C" self))
  (UserInterface|Viewport|AddtoViewport _returnvalue 0))

(fn WinGame
  (Widget|RemovefromParent (Variables|Default|GetConsoleUI))
  (bind _returnvalue (UserInterface|CreateWidget "/Game/Blueprints/UI/WBP_WinScreen.WBP_WinScreen_C" (Game|GetPlayerController 0)))
  (UserInterface|Viewport|AddtoViewport _returnvalue 0))

(fn ClearInputBuffer
  (Variables|Inputs|SetInputBuffered "NewEnumerator6")
  (Audio|Components|Audio|Stop (Variables|Default|GetInputBuffering)))

(fn SendMovementInput
  (params (Direction :type E_PlayerInput%20Enum :default "NewEnumerator6"))
  (Variables|Inputs|SetInputBuffered Direction)
  (Inputs|CheckInputBuffer))

(fn CheckInputBuffer
  (bind _asbpplayercharacter (CallFunction|GetPlayerCharacter))
  (Inputs|FetchPressedButton)
  (if (and (Utilities|Enum|NotEqual(Enum) (Variables|Inputs|GetInputBuffered) "NewEnumerator6") (Variables|/Game/Blueprints/BP_PlayerCharacter.BP_PlayerCharacter_C|GetCanPressMove (CallFunction|GetPlayerCharacter)))
    (Variables|/Game/Blueprints/BP_PlayerCharacter.BP_PlayerCharacter_C|SetCanPressMove (CallFunction|GetPlayerCharacter) false)
    (Utilities|FlowControl|Sequence
      (:then_0
        (switch Utilities|FlowControl|Switch|SwitchonE_PlayerInput (Variables|Inputs|GetInputBuffered)
          (:NewEnumerator0
            (Default|MoveForwards _asbpplayercharacter))
          (:NewEnumerator1
            (Default|MoveBackwards _asbpplayercharacter))
          (:NewEnumerator2
            (Default|MoveLeft _asbpplayercharacter))
          (:NewEnumerator3
            (Default|MoveRight _asbpplayercharacter))
          (:NewEnumerator4
            (Default|TurnLeft _asbpplayercharacter))
          (:NewEnumerator5
            (Default|TurnRight _asbpplayercharacter))))
      (:then_1
        (Development|PrintString (Utilities|String|EnumtoString (Variables|Inputs|GetInputBuffered))))
      (:then_2
        (Inputs|ClearInputBuffer)))
    (else
      (Components|Timeline|PlayfromStart (Variables|Default|GetInputBuffering)))))

(fn FetchPressedButton
  (if (Utilities|Enum|Equal(Enum) (Variables|Inputs|GetInputBuffered) "NewEnumerator6")
    (Variables|Inputs|SetInputBuffered (Default|GetCurrentlyPressedButton (Variables|Default|GetMovementUI)))))

(fn GetRestrictedMovements
  (Utilities|Array|Clear (LocalVariables|GetTmpForbiddenInputs))
  ;[0.15 0.15 0.15 0.5] Check each direction, if we hit a wall, add the direction to forbidden inputs
  (for _array_element (Utilities|Array|MakeArray "NewEnumerator0" "NewEnumerator1" "NewEnumerator2" "NewEnumerator3")
    (bind _hit (Default|CheckWallDirection (CallFunction|GetPlayerCharacter) _array_element))
    (if _hit
      (Utilities|Array|Add (LocalVariables|GetTmpForbiddenInputs) _array_element)))
  (return (LocalVariables|GetTmpForbiddenInputs)))

(fn FinishMovement
  (bind _forbiddeninputs (Inputs|GetRestrictedMovements))
  (Default|RestrictPlayerInputs (Variables|Default|GetMovementUI) _forbiddeninputs)
  (Inputs|CheckInputBuffer))

(fn HighlightPlayerInput
  (params (PlayerInput :type E_PlayerInput%20Enum :default "NewEnumerator6"))
  (Default|HighlightPlayerInput (Variables|Default|GetMovementUI) PlayerInput))

(fn FocusonInteractible
  (params (Interactible :type BP%20Interactible%20Object%20Reference))
  (bind _output_get (Variables|Default|SetCurrentInteractible Interactible))
  (Default|StartInteraction _output_get)
  (Game|Player|SetViewTargetwithBlend _output_get 0.5 "VTBlend_Linear" 0.0 false)
  (Widget|RemovefromParent (Variables|Default|GetMovementUI))
  (UserInterface|Viewport|AddtoViewport (Variables|Default|GetExitFocusUI) 0))

(fn ExitFocus
  (Default|EndInteraction (Variables|Default|GetCurrentInteractible))
  (Variables|Default|SetCurrentInteractible 0)
  (Game|Player|SetViewTargetwithBlend (CallFunction|GetPlayerCharacter) 0.5 "VTBlend_Linear" 0.0 false)
  (Widget|RemovefromParent (Variables|Default|GetExitFocusUI))
  (UserInterface|Viewport|AddtoViewport (Variables|Default|GetMovementUI) 0))

(fn ShowConsole
  (UserInterface|Viewport|AddtoViewport (Variables|Default|GetConsoleUI) 0)
  (Input|SetInputModeUIOnly self 0 "DoNotLock" false))

(fn HideConsole
  (Widget|RemovefromParent (Variables|Default|GetConsoleUI))
  (Input|SetInputModeGameandUI self 0 "DoNotLock" false false))

(fn InitExits
  (for _array_element (Variables|Exits|GetAvailableExits)
    (Utilities|Map|Add (Variables|Exits|GetExitsMap) (Variables|/Game/Blueprints/BP_Exit.BP_Exit_C|GetLocation _array_element) _array_element)))

(fn SpawnVfx
  (params (Vfx :type Niagara%20System%20Object%20Reference) (Location :type E_SymbolLocation%20Enum :default "NewEnumerator0"))
  (bind _exitsmap (Variables|Exits|GetExitsMap))
  (bind _value (Utilities|Map|Find _exitsmap Location))
  (bind _monsteranchor (Variables|/Game/Blueprints/BP_Exit.BP_Exit_C|GetMonsterAnchor _value))
  (Niagara|SpawnSystematLocation Vfx (Transformation|GetWorldLocation _monsteranchor) (Transformation|GetWorldRotation _monsteranchor) "1.000000,1.000000,1.000000" true true "None" false))